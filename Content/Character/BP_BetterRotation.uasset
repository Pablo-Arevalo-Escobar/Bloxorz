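; BP_BetterRotation is a player-driven cube that rotates 90 degrees in world space on move input.
; BeginPlay adds the Enhanced Input mapping context, and IA_Move, gated by a delay, accepts only exact positive X (pitch) or Y (roll).
; Tick applies a fixed per-frame step, unscaled by delta time, blocking new turns until finished.
; The final step always rolls, even for pitch turns.
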(event `self.ReceiveTick`
  (params (DeltaSeconds :type "Float (single-precision)"))
  (bind _cube (`self.Cube`))
  (if (`self.Rotating`)
    (if (> (`self.RotationToAdd`) (`self.RotationDelta`))
      (`KismetSystemLibrary.PrintString` (`KismetStringLibrary.Conv_DoubleToString` (`self.RotationDelta`)))
      (if (`self.AddingY`)
        (`SceneComponent.K2_AddWorldRotation` _cube (`KismetMathLibrary.MakeRotator` (`self.RotationDelta`)) false false)
        (else
          (`SceneComponent.K2_AddWorldRotation` _cube (`KismetMathLibrary.MakeRotator` 0.0 (`self.RotationDelta`)) false false)))
      (if (`self.AddingY`)
        (set `self.RotationToAdd` (- (`self.RotationToAdd`) (`self.RotationDelta`)))
        (else
          (set `self.RotationToAdd` (- (`self.RotationToAdd`) (`self.RotationDelta`)))))
      (else
        (if (`self.AddingY`)
          (`SceneComponent.K2_AddWorldRotation` (`self.Cube`) (`KismetMathLibrary.MakeRotator` (`self.RotationDelta`)) false false)
          (else
            (`SceneComponent.K2_AddWorldRotation` _cube (`KismetMathLibrary.MakeRotator` (`self.RotationToAdd`)) false false)))
        (set `self.Rotating` false)))))

(event `EnhancedInput|/Game/Character/Input/IA_Move`
  (params (ActionValue :type "Vector Structure") (ElapsedSeconds :type "Float (double-precision)") (TriggeredSeconds :type "Float (double-precision)") (InputAction :type "InputAction Object Reference" :default "/Game/Character/Input/IA_Move.IA_Move"))
  (:`Triggered`
    (if (> (- (`GameplayStatics.GetTimeSeconds`) (`self.TimeSinceLastInput`)) (`self.InputDelay`))
      (`|ExecutionSequence`
        (:`then_0`
          (if (and (== ActionValue (1.0 0.0 0.0)) (not (`self.Rotating`)))
            (set `self.AddingY` false)
            (set `self.Rotating` true :!label _label)
            (set `self.StartTime` (`GameplayStatics.GetTimeSeconds`))
            (set `self.RotationToAdd` 90.0)
            (bind _output_get (set `self.RotationDelta` (/ (`self.RotationToAdd`) (`self.RotationLength`))))
            (set `self.TimeSinceLastInput` (`GameplayStatics.GetTimeSeconds`))
            (`KismetSystemLibrary.PrintString` (`KismetStringLibrary.Conv_DoubleToString` _output_get))))
        (:`then_1`
          (if (and (== ActionValue (0.0 1.0 0.0)) (not (`self.Rotating`)))
            (set `self.AddingY` true)
            (goto _label)))))))

(event `self.ReceiveBeginPlay`
  (bind _asbp_player_controller (cast `/Game/Character/BP_PlayerController` (`GameplayStatics.GetPlayerController` 0)))
  (`EnhancedInputSubsystemInterface.AddMappingContext` (pcsubsystem `EnhancedInputLocalPlayerSubsystem` _asbp_player_controller) "/Game/Character/Input/MC_BloxCharacter.MC_BloxCharacter" 0 (struct)))

(fn `UserConstructionScript`)