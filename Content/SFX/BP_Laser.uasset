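; Laser beam effect actor that extends forward on spawn, stays on for a set time, then hides.
; BeginPlay tints the beam and impact Niagara systems and plays a charge sound at the world origin.
; Tick grows the beam's LaserEnd parameter over the startup time without collision checks.
; It then line-traces forward each frame to clip the beam and place the impact effect, until the on-time expires.
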(event `self.ReceiveBeginPlay`
  (`FXSystemComponent.SetColorParameter` (`self.NiagaraLaser`) "Color" (`KismetMathLibrary.Conv_ColorToLinearColor` (`self.LaserColor`)))
  (`FXSystemComponent.SetColorParameter` (`self.NiagaraLaserImpact`) "Color" (`KismetMathLibrary.Conv_ColorToLinearColor` (`self.LaserColor`)))
  (set `self.InStartup` true)
  (`FXSystemComponent.SetVectorParameter` (`self.NiagaraLaser`) "LaserEnd" (0.0 0.0 0.0))
  (set `self.StartupTime` (`GameplayStatics.GetTimeSeconds`))
  (`GameplayStatics.PlaySoundAtLocation` "/Game/SFX/Audio/EnergyGun_Charge1.EnergyGun_Charge1" (0.0 0.0 0.0) (struct) 1.0 1.0 0.0 null null null null))

(event `self.ReceiveTick`
  (params (DeltaSeconds :type "Float (single-precision)"))
  (bind _returnvalue (`self.K2_GetActorLocation`))
  (bind _returnvalue_2 (+ _returnvalue (* (`self.GetActorForwardVector`) (`self.Distance`))))
  (bind _returnvalue_3 (`KismetMathLibrary.FClamp` (/ (- (`GameplayStatics.GetTimeSeconds`) (`self.StartupTime`)) (`self.StartupLength`))))
  (if (`self.InStartup`)
    (`FXSystemComponent.SetVectorParameter` (`self.NiagaraLaser`) "LaserEnd" (+ (`self.K2_GetActorLocation`) (* (`self.GetActorForwardVector`) (`KismetMathLibrary.Lerp` 0.0 (`self.Distance`) _returnvalue_3))))
    (if (>= _returnvalue_3 1.0)
      (set `self.InStartup` false)
      (set `self.OnTime` (`GameplayStatics.GetTimeSeconds`)))
    (elif (> (- (`GameplayStatics.GetTimeSeconds`) (`self.OnTime`)) (`self.OnLength`))
      (`SceneComponent.SetVisibility` (`self.NiagaraLaserImpact`) false false)
      (`SceneComponent.SetVisibility` (`self.NiagaraLaser`) false false)
      (else
        (bind (_outhit _returnvalue_4) (`KismetSystemLibrary.LineTraceSingle` _returnvalue _returnvalue_2 "TraceTypeQuery1"))
        (bind (_bblockinghit _binitialoverlap _time _distance _location) (`GameplayStatics.BreakHitResult` _outhit))
        (`FXSystemComponent.SetVectorParameter` (`self.NiagaraLaser`) "LaserEnd" (`KismetMathLibrary.SelectVector` _location _returnvalue_2 _returnvalue_4))
        (if _returnvalue_4
          (`SceneComponent.K2_SetWorldLocation` (`self.NiagaraLaserImpact`) _location false false)
          (`SceneComponent.SetVisibility` (`self.NiagaraLaserImpact`) true false)
          (else
            (`SceneComponent.SetVisibility` (`self.NiagaraLaserImpact`) false false)))))))

(fn `UserConstructionScript`)