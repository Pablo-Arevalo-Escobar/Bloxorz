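; End tile actor for the grid, with tick disabled at BeginPlay.
; OnEndAnimation adds an audio component and schedules it to stop after a short delay.
; A disconnected, never-executed sequence would spawn four BP_Laser actors offset on each side of the tile, rotated to face different directions.
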(event `self.ReceiveBeginPlay`
  (`self.SetActorTickEnabled` false))

(event `self.OnEndAnimation`
  (bind _returnvalue (`AddComponent|NODE_AddAudioComponent-0`))
  (`AudioComponent.StopDelayed` _returnvalue 3.0))

(fn `UserConstructionScript`)