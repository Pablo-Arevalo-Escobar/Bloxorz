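; Game mode for the Blox game that sets up the player HUD and handles level completion and death.
; On BeginPlay it shows the HUD with mouse input, caches BP_BloxGameInstance and stores the level number parsed from the map name.
; OnLevelEnd advances the level and commits the move count, while OnDeath resets that level's moves.
; Both play a transition widget, then open the level named by the game instance.
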(event `self.ReceiveBeginPlay`
  (bind _returnvalue (`GameplayStatics.GetPlayerController` 0))
  (`|ExecutionSequence`
    (:`then_0`
      ;[1 1 1] Create and Initialize HUD Widget
      (bind _returnvalue_2 (`|CreateWidget` "/Game/Blueprints/Widgets/Menu/W_PlayerHud.W_PlayerHud_C"))
      (bind _output_get (set `self.HUD` _returnvalue_2))
      (`UserWidget.AddToViewport` _output_get 0)
      (`WidgetBlueprintLibrary.SetInputMode_GameAndUIEx` _returnvalue _output_get "LockAlways" false)
      (set `PlayerController.bShowMouseCursor` true _returnvalue))
    (:`then_1`
      ;[1 1 1] Store Game Instance
      (bind _asbp_blox_game_instance (cast `/Game/BP_BloxGameInstance` (`GameplayStatics.GetGameInstance`)))
      (set `self.GameInstance` _asbp_blox_game_instance))
    (:`then_2`
      ;[1 1 1] Store current level name
      (bind _returnvalue_3 (`GameplayStatics.GetCurrentLevelName` true))
      (set `/Game/BP_BloxGameInstance.CurrentLevel` (`KismetStringLibrary.Conv_StringToInt` (`KismetStringLibrary.GetSubstring` _returnvalue_3 3 (`KismetMathLibrary.Min` (`KismetStringLibrary.Len` _returnvalue_3) 3))) (`self.GameInstance`)))))

(event `self.OnLevelEnd`
  (`/Game/BP_BloxGameInstance.IncrementCurrentLevel` (`self.GameInstance`))
  (bind _returnvalue (`|CreateWidget` "/Game/Blueprints/Widgets/W_Transition.W_Transition_C"))
  (`UserWidget.AddToViewport` _returnvalue 0)
  ;[1 1 1] Save the number of moves made by the player
  (`BloxGameInstance.ApplyMoveDelta` (`self.GameInstance`))
  (`KismetSystemLibrary.Delay` 0.5)
  (bind _levelname (`/Game/BP_BloxGameInstance.Get Level ID` (`self.GameInstance`)))
  (set `self.Level Name` _levelname)
  (`GameplayStatics.OpenLevel` _levelname))

(event `self.OnDeath`
  (`KismetSystemLibrary.Delay` 1.0)
  (bind _returnvalue (`|CreateWidget` "/Game/Blueprints/Widgets/W_Transition.W_Transition_C"))
  (`UserWidget.AddToViewport` _returnvalue 0)
  ;[1 1 1] Reset number of moves made by the player this level
  (`BloxGameInstance.ResetMoveDelta` (`self.GameInstance`))
  (`KismetSystemLibrary.Delay` 0.5)
  (bind _levelname (`/Game/BP_BloxGameInstance.Get Level ID` (`self.GameInstance`)))
  (`GameplayStatics.OpenLevel` _levelname)
  (`KismetSystemLibrary.PrintString` "Hello"))

(fn `UserConstructionScript`)